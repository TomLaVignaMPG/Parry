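; Moving platform actor that shuttles between two points and can be switched on and off through bound activate and deactivate events tied to a pressure reference.
; It starts at Point1, and chained MoveComponentTo nodes with a FlipFlop loop it, pausing at Point2.
; Activation turns the edge glow green and starts movement.
; Deactivation turns it red, clears the Activate flag and reverses the outbound move.
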(event `self.ReceiveBeginPlay`
  (bind _easein (`self.EaseIn`))
  (bind _easein_2 (`self.EaseIn`))
  (add `self.ActivatePlatform` (delegate `Active`))
  (add `self.DeactivatePlatform` (delegate `Deactive`))
  (`SceneComponent.K2_SetWorldLocation` (`self.Platform`) (`SceneComponent.K2_GetComponentLocation` (`self.Point1`)) false false)
  (if (`self.Activate`)
    (`PrimitiveComponent.SetMaterial` (`self.Edge Glow`) 0 "/Game/Blueprints/Materials/Green.Green")
    (`KismetSystemLibrary.MoveComponentTo` (`self.Platform`) (`SceneComponent.RelativeLocation` (`self.Point2`)) (struct) _easein_2 _easein_2 (`self.MoveTime`) :!label _label)
    (`KismetSystemLibrary.Delay` (`self.PauseTime`))
    (if (`self.Activate`)
      (`/Engine/EditorBlueprintResources/StandardMacros.FlipFlop` :!label _label_2
        (:`A`
          (`KismetSystemLibrary.MoveComponentTo` (`self.Platform`) (`SceneComponent.RelativeLocation` (`self.Point1`)) (struct) _easein _easein (`self.MoveTime`) :!label _label_3)
          (goto _label_2))
        (:`B`
          (goto _label)))
      (else
        (goto _label_3 :!via `Return`)))
    (else
      (`PrimitiveComponent.SetMaterial` (`self.Edge Glow`) 0 "/Game/Blueprints/Materials/Red.Red" :!label _label_4)
      (set `self.Activate` false)
      (goto _label :!via `Return`))))

(event `Deactive`
  (`/Game/Blueprints/Actors/PressurePad.ResetActivation` (`self.PressureReference`))
  (goto _label_4))

(event `Active`
  (`PrimitiveComponent.SetMaterial` (`self.Edge Glow`) 0 "/Game/Blueprints/Materials/Green.Green")
  (`/Game/Blueprints/Actors/PressurePad.ResetDeactivation` (`self.PressureReference`))
  (goto _label))

(fn `UserConstructionScript`)