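; Pressure pad actor that activates two referenced platforms and opens a referenced door when the player overlaps its box.
; A DoOnce gates activation, turning the glow green until ResetActivation re-arms it.
; End overlap does nothing, and the second DoOnce's entry is disconnected, so the red glow and platform deactivation never run, as ResetDeactivation only resets that gate.
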(event `self.Box.OnComponentBeginOverlap`
  (params (OverlappedComponent :type "PrimitiveComponent Object Reference") (OtherActor :type "Actor Object Reference") (OtherComp :type "PrimitiveComponent Object Reference") (OtherBodyIndex :type Integer) (bFromSweep :type Boolean) (SweepResult :type "HitResult Structure (by ref)"))
  (cast `/Game/Blueprints/Characters/BP_Player` OtherActor)
  (`/Engine/EditorBlueprintResources/StandardMacros.DoOnce` false :!label _label
    (:`Completed`
      (`PrimitiveComponent.SetMaterial` (`self.Glow`) 0 "/Game/Blueprints/Materials/Green.Green")
      (`/Game/Blueprints/Actors/BP_MovingPlatform.ActivatePlatform` (`self.PlatformReference`))
      (`/Game/Blueprints/Actors/BP_MovingPlatform.ActivatePlatform` (`self.PlatformReference2`))
      (`/Game/Blueprints/Actors/BP_Door.OnOpened` (`self.DoorReference`)))))

(event `ResetActivation`
  (goto _label :!via `Reset`))

(event `self.Box.OnComponentEndOverlap`
  (params (OverlappedComponent :type "PrimitiveComponent Object Reference") (OtherActor :type "Actor Object Reference") (OtherComp :type "PrimitiveComponent Object Reference") (OtherBodyIndex :type Integer)))

(event `ResetDeactivation`
  (`/Engine/EditorBlueprintResources/StandardMacros.DoOnce` false :!via `Reset`
    (:`Completed`
      (`PrimitiveComponent.SetMaterial` (`self.Glow`) 0 "/Game/Blueprints/Materials/Red.Red")
      (`/Game/Blueprints/Actors/BP_MovingPlatform.DeactivatePlatform` (`self.PlatformReference`))
      (`/Game/Blueprints/Actors/BP_MovingPlatform.DeactivatePlatform` (`self.PlatformReference2`)))))

(fn `UserConstructionScript`)