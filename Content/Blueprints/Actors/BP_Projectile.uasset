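; BP_Projectile is a homing projectile that damages the player and can be deflected back to damage a BP_FireDemon.
; DamageBox handles the first hit, damaging the player or simply destroying the projectile on other actors.
; ProjectileTakeDamage retargets homing to the original instigator, records the new one, and swaps collision from DamageBox to DeflectBox.
; DeflectBox then damages an overlapped fire demon and destroys the projectile; the health-change handler is empty.
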(event `self.ReceiveBeginPlay`
  (add `PA_Health.OnHealthChanged` (`self.PA_Health`) (`|CreateDelegate` :!event `HandleOnHealthChanged`))
  (`PrimitiveComponent.SetCollisionEnabled` (`self.DeflectBox`) "NoCollision")
  (set `self.SpawnLocation` (`self.K2_GetActorLocation`))
  (set `ProjectileMovementComponent.HomingTargetComponent` (`Actor.RootComponent` (`self.HomingTargetComponent`)) (`self.ProjectileMovement`)))

(event `self.ReceiveTick`
  (params (DeltaSeconds :type "Float (single-precision)"))
  (if (`self.IsDead`)
    (`self.K2_DestroyActor`)))

(event `self.DamageBox.OnComponentBeginOverlap`
  (params (OverlappedComponent :type "PrimitiveComponent Object Reference") (OtherActor :type "Actor Object Reference") (OtherComp :type "PrimitiveComponent Object Reference") (OtherBodyIndex :type Integer) (bFromSweep :type Boolean) (SweepResult :type "HitResult Structure (by ref)"))
  (`self.HurtPlayer` OtherActor OtherActor))

(event `self.PA_Health.OnHealthChanged`
  (params (HealthDelta :type "Float (single-precision)") (CurrentHealth :type "Float (single-precision)"))
  (`self.HandleOnHealthChanged` HealthDelta CurrentHealth))

(event `self.DeflectBox.OnComponentBeginOverlap`
  (params (OverlappedComponent :type "PrimitiveComponent Object Reference") (OtherActor :type "Actor Object Reference") (OtherComp :type "PrimitiveComponent Object Reference") (OtherBodyIndex :type Integer) (bFromSweep :type Boolean) (SweepResult :type "HitResult Structure (by ref)"))
  (bind _asbp_fire_demon (cast `/Game/Blueprints/Characters/BP_FireDemon` OtherActor))
  (`/Game/Blueprints/Characters/BP_FireDemon.DemonTakeDamage` _asbp_fire_demon (`self.BaseDamage`))
  (`self.K2_DestroyActor`))

(fn `HandleOnHealthChanged`
  (params (HealthDelta :type "Float (single-precision)") (CurrentHealth :type "Float (single-precision)")))

(fn `HurtPlayer`
  (params (Object :type "Object Object Reference") (A :type "Object Object Reference"))
  (`/Engine/EditorBlueprintResources/StandardMacros.DoOnce` false
    (:`Completed`
      (if (`self.IsDeflected`)
        _
        (elif (`self.IsDead`)
          _
          (elif (== A (`GameplayStatics.GetPlayerCharacter` 0))
            (bind _asbp_player (cast `/Game/Blueprints/Characters/BP_Player` Object))
            (`/Game/Blueprints/Characters/BP_Player.TakeDamage` _asbp_player (`self.BaseDamage`))
            (`self.K2_DestroyActor`)
            (else
              (`self.K2_DestroyActor`))))))))

(fn `ProjectileTakeDamage`
  (params (`Health Changed` :type "Float (double-precision)") (DamageInstigator :type "Pawn Object Reference"))
  (set `ProjectileMovementComponent.HomingTargetComponent` (`Actor.RootComponent` (`self.Instigator`)) (`self.ProjectileMovement`))
  (set `self.Instigator` DamageInstigator)
  (`PrimitiveComponent.SetCollisionEnabled` (`self.DeflectBox`) "QueryOnly")
  (`PrimitiveComponent.SetCollisionEnabled` (`self.DamageBox`) "NoCollision"))

(fn `UserConstructionScript`)