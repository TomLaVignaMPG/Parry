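; A breakable platform actor that collapses after BP_Player hits it, then returns to its start location.
; The hit passes through a DoOnce before the player cast, then starts a timer.
; Tick uses nested time thresholds to tilt the platform, sink it per frame, disable collision and hide it.
; Once the timer ends, Tick restores collision, visibility and position, and resets the DoOnce.
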(event `self.ReceiveBeginPlay`
  (set `self.StartLocation` (`self.K2_GetActorLocation`)))

(event `self.Platform.OnComponentHit`
  (params (HitComponent :type "PrimitiveComponent Object Reference") (OtherActor :type "Actor Object Reference") (OtherComp :type "PrimitiveComponent Object Reference") (NormalImpulse :type "Vector Structure") (Hit :type "HitResult Structure (by ref)"))
  (`/Engine/EditorBlueprintResources/StandardMacros.DoOnce` false :!label _label
    (:`Completed`
      (cast `/Game/Blueprints/Characters/BP_Player` OtherActor)
      (set `self.IsBreaking` true)
      (set `self.TimeSinceStartBreaking` 0.0))))

(event `Reset Platform`
  (goto _label :!via `Reset`))

(event `self.ReceiveTick`
  (params (DeltaSeconds :type "Float (single-precision)"))
  (if (`self.IsBreaking`)
    (set `self.TimeSinceStartBreaking` (+ (`self.TimeSinceStartBreaking`) DeltaSeconds))
    (if (>= (`self.TimeSinceStartBreaking`) 0.5)
      (`self.K2_SetActorRotation` (struct :`Pitch` 10.0))
      (if (>= (`self.TimeSinceStartBreaking`) 1.0)
        (`self.K2_SetActorRotation` (struct :`Pitch` -10.0))
        (if (>= (`self.TimeSinceStartBreaking`) 2.0)
          (`self.K2_SetActorTransform` (`KismetMathLibrary.Conv_VectorToTransform` (- (`self.K2_GetActorLocation`) (0.0 0.0 1.0))))
          (if (>= (`self.TimeSinceStartBreaking`) 3.0)
            (`PrimitiveComponent.SetCollisionEnabled` (`self.Platform`) "NoCollision")
            (`KismetSystemLibrary.Delay` 0.2)
            (`self.SetActorHiddenInGame` true)
            (if (>= (`self.TimeSinceStartBreaking`) 6.0)
              (set `self.IsBreaking` false))))))
    (elif (>= (`self.TimeSinceStartBreaking`) 6.0)
      (`PrimitiveComponent.SetCollisionEnabled` (`self.Platform`) "QueryAndPhysics")
      (`self.SetActorHiddenInGame` false)
      (`self.K2_SetActorTransform` (`KismetMathLibrary.Conv_VectorToTransform` (`self.StartLocation`)))
      (`self.Reset Platform`))))

(fn `UserConstructionScript`)