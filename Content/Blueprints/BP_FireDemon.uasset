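; BP_FireDemon is a flipbook-animated enemy that turns to face the player along X and fires homing projectiles.
; A looping timer spawns a BP_Projectile targeting the player, only while alive and when no previous projectile is still valid.
; A PAHealth component takes damage, with handlers that switch flipbooks and set Hurt or IsDead.
; Once dead, Tick destroys the capsule, then the actor after a short delay.
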(event `self.ReceiveBeginPlay`
  (add `PA_Health.OnHealthChanged` (`self.PA_Health`) (`|CreateDelegate` :!event `HandleOnHealthChanged`))
  (add `PA_Health.OnDeath` (`self.PA_Health`) (`|CreateDelegate` :!event `HandleOnDeath`))
  (`KismetSystemLibrary.K2_SetTimerDelegate` (delegate `Shoot Projectile`) (`self.Time`) true))

(event `Shoot Projectile`
  (if (not (`self.Is Dead`))
    (`self.CheckProjectile`)))

(event `self.PA_Health.OnHealthChanged`
  (params (HealthDelta :type "Float (single-precision)") (CurrentHealth :type "Float (single-precision)"))
  (`self.HandleOnHealthChanged` HealthDelta CurrentHealth))

(event `self.ReceiveTick`
  (params (DeltaSeconds :type "Float (single-precision)"))
  (`self.FacePlayer`)
  (if (`self.Is Dead`)
    (`/Engine/EditorBlueprintResources/StandardMacros.IsValid` (`self.CapsuleComponent`)
      (:`Is Valid`
        (`ActorComponent.K2_DestroyComponent` (`self.CapsuleComponent`))
        (`KismetSystemLibrary.Delay` 0.2)
        (`self.K2_DestroyActor`)))))

(fn `CheckProjectile`
  (if (not (`KismetSystemLibrary.IsValid` (`self.Projectile`)))
    (`self.CreateProjectile`)))

(fn `CreateProjectile`
  (bind _returnvalue (`|SpawnActorFromClass` "/Game/Blueprints/BP_Projectile.BP_Projectile_C" (`KismetMathLibrary.MakeTransform` (`self.K2_GetActorLocation`)) "AlwaysSpawn" "MultiplyWithRoot" self (`GameplayStatics.GetPlayerCharacter` 0) self))
  (set `self.Projectile` _returnvalue))

(fn `DemonTakeDamage`
  (params (DamageAmount :type "Float (double-precision)"))
  (`PA_Health.ChangeHealth` (`self.PA_Health`) DamageAmount))

(fn `FacePlayer`
  (bind _returnvalue_x (`KismetMathLibrary.BreakVector` (`self.K2_GetActorLocation`)))
  (bind _returnvalue_x_2 (`KismetMathLibrary.BreakVector` (`self.K2_GetActorLocation` (`GameplayStatics.GetPlayerCharacter` 0))))
  (if (> (- _returnvalue_x_2 _returnvalue_x) 0.0)
    (`self.K2_SetActorRotation` (struct :`Yaw` 180.0))
    (else
      (`self.K2_SetActorRotation` (struct)))))

(fn `HandleOnDeath`
  (`PaperFlipbookComponent.SetFlipbook` (`self.Sprite`) "/Game/PaperAssets/FireDemon/FB_FireDemon_Death.FB_FireDemon_Death")
  (`PaperFlipbookComponent.SetLooping` (`self.Sprite`) false)
  (set `self.Is Dead` true))

(fn `HandleOnHealthChanged`
  (params (HealthDelta :type "Float (single-precision)") (CurrentHealth :type "Float (single-precision)"))
  (`PaperFlipbookComponent.SetFlipbook` (`self.Sprite`) null)
  (`PaperFlipbookComponent.SetLooping` (`self.Sprite`) false)
  (set `self.Hurt` true))

(fn `UserConstructionScript`)