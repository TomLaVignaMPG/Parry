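; BP_Wizard is a flipbook-animated enemy that faces the player and periodically casts fire walls.
; A looping timer spawns BP_FireWall at its location until it dies, while Tick flips its rotation by the player's X position.
; PAHealth events switch Hurt and Death flipbooks, returning to Idle when a non-death animation finishes.
; Once IsDead is set, Tick removes the capsule and destroys the actor after a short delay.
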(event `self.ReceiveBeginPlay`
  (add `PA_Health.OnHealthChanged` (`self.PA_Health`) (`|CreateDelegate` :!event `HandleOnHealthChanged`))
  (add `PA_Health.OnDeath` (`self.PA_Health`) (`|CreateDelegate` :!event `HandleOnDeath`))
  (`KismetSystemLibrary.K2_SetTimerDelegate` (delegate `Shoot Projectile`) (`self.Time`) true))

(event `Shoot Projectile`
  (if (not (`self.Is Dead`))
    (`self.CreateWall`)))

(event `self.ReceiveTick`
  (params (DeltaSeconds :type "Float (single-precision)"))
  (`self.FacePlayer`)
  (if (`self.Is Dead`)
    (`/Engine/EditorBlueprintResources/StandardMacros.IsValid` (`self.CapsuleComponent`)
      (:`Is Valid`
        (`ActorComponent.K2_DestroyComponent` (`self.CapsuleComponent`))
        (`KismetSystemLibrary.Delay` 1.0)
        (`self.K2_DestroyActor`)))))

(event `self.PA_Health.OnHealthChanged`
  (params (HealthDelta :type "Float (single-precision)") (CurrentHealth :type "Float (single-precision)"))
  (`self.HandleOnHealthChanged` HealthDelta CurrentHealth))

(event `self.Sprite.OnFinishedPlaying`
  (if (not (`self.Is Dead`))
    (`PaperFlipbookComponent.SetFlipbook` (`self.Sprite`) "/Game/PaperAssets/Wizard/Flipbooks/FB_Wizard_Idle.FB_Wizard_Idle")
    (`self.RestartAnimation`)))

(fn `CreateWall`
  (bind _returnvalue (`|SpawnActorFromClass` "/Game/Blueprints/BP_FireWall.BP_FireWall_C" (`KismetMathLibrary.MakeTransform` (`self.K2_GetActorLocation`) (`self.K2_GetActorRotation`)) "AlwaysSpawn" "MultiplyWithRoot" null self))
  (set `self.Wall` _returnvalue))

(fn `FacePlayer`
  (bind _returnvalue_x (`KismetMathLibrary.BreakVector` (`self.K2_GetActorLocation`)))
  (bind _returnvalue_x_2 (`KismetMathLibrary.BreakVector` (`self.K2_GetActorLocation` (`GameplayStatics.GetPlayerCharacter` 0))))
  (if (> (- _returnvalue_x_2 _returnvalue_x) 0.0)
    (`self.K2_SetActorRotation` (struct :`Yaw` 180.0))
    (else
      (`self.K2_SetActorRotation` (struct)))))

(fn `HandleOnDeath`
  (`PaperFlipbookComponent.SetFlipbook` (`self.Sprite`) "/Game/PaperAssets/Wizard/Flipbooks/FB_Wizard_Death.FB_Wizard_Death")
  (`PaperFlipbookComponent.SetLooping` (`self.Sprite`) false)
  (set `self.Is Dead` true))

(fn `HandleOnHealthChanged`
  (params (HealthDelta :type "Float (single-precision)") (CurrentHealth :type "Float (single-precision)"))
  (`PaperFlipbookComponent.SetFlipbook` (`self.Sprite`) "/Game/PaperAssets/Wizard/Flipbooks/FB_Wizard_Hurt.FB_Wizard_Hurt")
  (`PaperFlipbookComponent.SetLooping` (`self.Sprite`) false)
  (set `self.Hurt` true))

(fn `RestartAnimation`
  (`PaperFlipbookComponent.SetLooping` (`self.Sprite`) true)
  (if (not (`PaperFlipbookComponent.IsPlaying` (`self.Sprite`)))
    (`PaperFlipbookComponent.Play` (`self.Sprite`))))

(fn `UserConstructionScript`)

(fn `WizardTakeDamage`
  (params (`Damage Amount` :type "Float (double-precision)"))
  (`PA_Health.ChangeHealth` (`self.PA_Health`) `Damage Amount`))