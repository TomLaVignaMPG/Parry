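; BP_Golem is a flipbook-animated melee enemy that chases and attacks the player within sight range.
; Tick selects attack or movement, using a forward-down trace against "Void" to avoid falls.
; Attack flipbook frames drive the player's parry window and damage, then a timer-based cooldown; parries trigger a knockback impulse.
; PA_Health events drive hurt stun and death cleanup, while homing-projectile helpers exist but are never called here.
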(event `self.ReceiveBeginPlay`
  (add `PA_Health.OnHealthChanged` (`self.PA_Health`) (`|CreateDelegate` :!event `HandleOnHealthChanged`))
  (add `PA_Health.OnDeath` (`self.PA_Health`) (`|CreateDelegate` :!event `HandleOnDeath`))
  (add `self.OnParried` (`|CreateDelegate` :!event `HandleOnParried`)))

(event `self.ReceiveTick`
  (params (DeltaSeconds :type "Float (single-precision)"))
  (if (`self.Hurt`)
    (`KismetSystemLibrary.Delay` 0.5)
    (set `self.Hurt` false)
    (elif (not (`self.Is Dead`))
      (if (not (`self.InAttackCooldown`))
        (bind _returnvalue (`self.DistanceToPlayer`))
        (if _returnvalue
          (`self.UpdateAttacking`)
          (elif (> (`self.RangeOfSight`) (`self.GetDistanceToPlayer`))
            (set `self.StopDamage` false)
            (if (not (`self.InAttackCooldown`))
              (`self.UpdateMovement`)))))
      (else
        (`/Engine/EditorBlueprintResources/StandardMacros.IsValid` (`self.CapsuleComponent`)
          (:`Is Valid`
            (`ActorComponent.K2_DestroyComponent` (`self.CapsuleComponent`))
            (`KismetSystemLibrary.Delay` 1.0)
            (`self.K2_DestroyActor`)))))))

(event `self.PA_Health.OnHealthChanged`
  (params (HealthDelta :type "Float (single-precision)") (CurrentHealth :type "Float (single-precision)"))
  (`self.HandleOnHealthChanged` HealthDelta CurrentHealth))

(event `self.Sprite.OnFinishedPlaying`
  (if (not (`self.Is Dead`))
    (`PaperFlipbookComponent.SetFlipbook` (`self.Sprite`) "/Game/PaperAssets/Golems_Free_Version/Golem_1/Blue/No_Swoosh_VFX/Flipbooks/FB_Golem_Idle.FB_Golem_Idle")
    (`self.Restart Animation`)
    (set `self.Attacking` false)))

(fn `CheckProjectile`
  (if (not (`KismetSystemLibrary.IsValid` (`self.Projectile`)))
    (`self.Create Projectile`)))

(fn `Create Projectile`
  (bind _returnvalue (`|SpawnActorFromClass` "/Game/Blueprints/BP_Projectile.BP_Projectile_C" (`KismetMathLibrary.MakeTransform` (`self.K2_GetActorLocation`)) "AlwaysSpawn" "MultiplyWithRoot" self (`GameplayStatics.GetPlayerCharacter` 0) self))
  (set `self.Projectile` _returnvalue))

(fn `DamagePlayer`
  (if (`self.bParried`)
    _
    (elif (`self.HitPlayer`)
      (`/Game/Blueprints/BP_Player.TakeDamage` (`self.CurrentPlayer`) (`self.Base Damage`))
      (set `self.HitPlayer` false))))

(fn `DistanceToPlayer`
  (returns (ReturnValue :type Boolean))
  (return (or (< (`self.GetDistanceToPlayer`) (`self.RangeOfAttack`)) (`self.WindUp`))))

(fn `EndOfAttackCooldown`
  (set `self.InAttackCooldown` false))

(fn `GetDistanceToPlayer`
  (returns (Result :type "Float (double-precision)"))
  (if (not (`KismetSystemLibrary.IsValid` (`self.CurrentPlayer`)))
    (bind _asbp_player (cast `/Game/Blueprints/BP_Player` (`GameplayStatics.GetPlayerCharacter` 0)))
    (set `self.CurrentPlayer` _asbp_player))
  (return (`KismetMathLibrary.Vector_Distance` (`self.K2_GetActorLocation`) (`self.K2_GetActorLocation` (`self.CurrentPlayer`)))))

(fn `GetPlayerLocation`
  (returns (ReturnValue :type "Vector Structure"))
  (if (`KismetSystemLibrary.IsValid` (`self.CurrentPlayer`))
    (return (`self.K2_GetActorLocation` (`self.CurrentPlayer`)))
    (else
      (bind _asbp_player (cast `/Game/Blueprints/BP_Player` (`GameplayStatics.GetPlayerCharacter` 0))
        (:`then`
          (bind _output_get (set `self.CurrentPlayer` _asbp_player))
          (return (`self.K2_GetActorLocation` _output_get)))
        (:`CastFailed`
          (return (0.0 0.0 0.0)))))))

(fn `GolemTakeDamage`
  (params (DamageAmount :type "Float (double-precision)"))
  (`PA_Health.ChangeHealth` (`self.PA_Health`) DamageAmount)
  (set `self.bParried` false))

(fn `HandleOnDeath`
  (`PaperFlipbookComponent.SetFlipbook` (`self.Sprite`) "/Game/PaperAssets/Golems_Free_Version/Golem_1/Blue/No_Swoosh_VFX/Flipbooks/FB_Golem_Death.FB_Golem_Death")
  (`PaperFlipbookComponent.SetLooping` (`self.Sprite`) false)
  (set `self.Is Dead` true))

(fn `HandleOnHealthChanged`
  (params (HealthDelta :type "Float (single-precision)") (CurrentHealth :type "Float (single-precision)"))
  (`PaperFlipbookComponent.SetFlipbook` (`self.Sprite`) "/Game/PaperAssets/Golems_Free_Version/Golem_1/Blue/No_Swoosh_VFX/Flipbooks/FB_Golem_Hurt.FB_Golem_Hurt")
  (`PaperFlipbookComponent.SetLooping` (`self.Sprite`) false)
  (set `self.Hurt` true))

(fn `HandleOnParried`
  (params (Parried :type Boolean) (Knockback :type "Float (single-precision)"))
  (bind (_returnvalue_roll _returnvalue_pitch _returnvalue_yaw) (`KismetMathLibrary.BreakRotator` (`self.K2_GetActorRotation`)))
  (set `self.bParried` Parried)
  (`PaperFlipbookComponent.SetFlipbook` (`self.Sprite`) "/Game/PaperAssets/Golems_Free_Version/Golem_1/Blue/No_Swoosh_VFX/Flipbooks/FB_Golem_Idle.FB_Golem_Idle")
  (if (> _returnvalue_yaw 90.0)
    (`CharacterMovementComponent.AddImpulse` (`self.CharacterMovement`) (+ (`self.K2_GetActorLocation`) (`KismetMathLibrary.MakeVector` Knockback)) true)
    (else
      (bind _result (`/Engine/EditorBlueprintResources/StandardMacros.NegateFloat` Knockback)
        (:`  `
          (`CharacterMovementComponent.AddImpulse` (`self.CharacterMovement`) (+ (`self.K2_GetActorLocation`) (`KismetMathLibrary.MakeVector` _result)) true))))))

(fn `MovementAndRotation`
  (params (Condition :type Boolean))
  (bind _returnvalue_x (`KismetMathLibrary.BreakVector` (`self.K2_GetActorLocation`)))
  (bind _returnvalue_x_2 (`KismetMathLibrary.BreakVector` (`self.K2_GetActorLocation` (`GameplayStatics.GetPlayerCharacter` 0))))
  (if (not Condition)
    (`self.AddMovementInput` (- (`self.GetPlayerLocation`) (`self.K2_GetActorLocation`))))
  (if (> (- _returnvalue_x_2 _returnvalue_x) 0.0)
    (`self.K2_SetActorRotation` (struct))
    (else
      (`self.K2_SetActorRotation` (struct :`Yaw` 180.0))))
  (if (not (== (`self.GetVelocity`) (0.0 0.0 0.0)))
    (`PaperFlipbookComponent.SetFlipbook` (`self.Sprite`) "/Game/PaperAssets/Golems_Free_Version/Golem_1/Blue/No_Swoosh_VFX/Flipbooks/FB_Golem_Walk.FB_Golem_Walk")
    (else
      (`PaperFlipbookComponent.SetFlipbook` (`self.Sprite`) "/Game/PaperAssets/Golems_Free_Version/Golem_1/Blue/No_Swoosh_VFX/Flipbooks/FB_Golem_Idle.FB_Golem_Idle"))))

(fn `PreventFalling`
  (returns (ReturnValue :type Boolean))
  (bind (_returnvalue_roll _returnvalue_pitch _returnvalue_yaw) (`KismetMathLibrary.BreakRotator` (`self.K2_GetActorRotation`)))
  (if (> _returnvalue_yaw 90.0)
    (set `self.Facing` 100.0)
    (else
      (set `self.Facing` -100.0)))
  (bind (_outhit _returnvalue) (`KismetSystemLibrary.LineTraceSingleByProfile` (`self.K2_GetActorLocation`) (+ (`self.K2_GetActorLocation`) (`KismetMathLibrary.MakeVector` (* (`self.Facing`) -1.0) 0.0 -500.0)) "Void"))
  (return _returnvalue))

(fn `Restart Animation`
  (`PaperFlipbookComponent.SetLooping` (`self.Sprite`) true)
  (if (not (`PaperFlipbookComponent.IsPlaying` (`self.Sprite`)))
    (`PaperFlipbookComponent.Play` (`self.Sprite`))))

(fn `UpdateAttacking`
  (bind _returnvalue (`PaperFlipbookComponent.GetPlaybackPositionInFrames` (`self.Sprite`)))
  (if (== (`PaperFlipbookComponent.GetFlipbook` (`self.Sprite`)) "/Game/PaperAssets/Golems_Free_Version/Golem_1/Blue/No_Swoosh_VFX/Flipbooks/FB_Golem_Attack.FB_Golem_Attack")
    (if (== (`PaperFlipbookComponent.GetPlaybackPositionInFrames` (`self.Sprite`)) 10)
      (bind _asbp_player (cast `/Game/Blueprints/BP_Player` (`GameplayStatics.GetPlayerCharacter` 0)))
      (set `/Game/Blueprints/BP_Player.ParryWindow` false _asbp_player)
      (set `self.WindUp` false)
      (set `self.InAttackCooldown` true)
      (`PaperFlipbookComponent.SetFlipbook` (`self.Sprite`) "/Game/PaperAssets/Golems_Free_Version/Golem_1/Blue/No_Swoosh_VFX/Flipbooks/FB_Golem_Idle.FB_Golem_Idle")
      (`self.AddMovementInput` (0.0 0.0 0.0))
      (set `self.Attacking` false)
      (`KismetSystemLibrary.K2_SetTimer` null "EndOfAttackCooldown" (`self.AttackCooldown`))
      (else
        (if (and (>= _returnvalue 6) (<= _returnvalue 9)) :!label _label
          (bind _asbp_player_2 (cast `/Game/Blueprints/BP_Player` (`GameplayStatics.GetPlayerCharacter` 0)))
          (set `/Game/Blueprints/BP_Player.ParryWindow` true _asbp_player_2)
          (`KismetSystemLibrary.PrintString` (`KismetStringLibrary.Conv_IntToString` (`PaperFlipbookComponent.GetPlaybackPositionInFrames` (`self.Sprite`))))
          (if (`self.bParried`)
            _
            (elif (< (`self.GetDistanceToPlayer`) (`self.RangeOfAttack`))
              (if (not (`self.Attacking`))
                (`/Game/Blueprints/BP_Player.TakeDamage` (`self.CurrentPlayer`) (`self.Base Damage`))
                (set `self.Attacking` true)))))))
    (else
      (`PaperFlipbookComponent.SetFlipbook` (`self.Sprite`) "/Game/PaperAssets/Golems_Free_Version/Golem_1/Blue/No_Swoosh_VFX/Flipbooks/FB_Golem_Attack.FB_Golem_Attack")
      (`PaperFlipbookComponent.SetLooping` (`self.Sprite`) false)
      (set `self.WindUp` true)
      (goto _label))))

(fn `UpdateMovement`
  (locals (NewLocalVar :type "Array of EObjectTypeQuery Enum") (NewLocalVar_0 :type "Float (double-precision)" :default 500.0))
  (bind _returnvalue (`self.PreventFalling`))
  (`self.MovementAndRotation` _returnvalue))

(fn `UserConstructionScript`)