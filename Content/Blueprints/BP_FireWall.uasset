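; BP_FireWall is a moving hazard that travels along its local negative X and damages the player on touch.
; The first DamageBox overlap passes a DoOnce, and if it is the player's BP_Player, the wall applies BaseDamage and destroys itself.
; Tick destroys it once dead or 800 units from its start on world X.
; WallTakeDamage changes PAHealth and marks it dead on any hit; the health-changed handler is empty.
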(event `self.ReceiveBeginPlay`
  (bind _returnvalue_x (`KismetMathLibrary.BreakVector` (`self.K2_GetActorLocation`)))
  (add `PA_Health.OnHealthChanged` (`self.PA_Health`) (`|CreateDelegate` :!event `HandleOnHealthChanged`))
  (set `self.Start location` _returnvalue_x)
  (`ProjectileMovementComponent.SetVelocityInLocalSpace` (`self.ProjectileMovement`) (-100.0 0.0 0.0)))

(event `self.ReceiveTick`
  (params (DeltaSeconds :type "Float (single-precision)"))
  (bind _returnvalue_x (`KismetMathLibrary.BreakVector` (`self.K2_GetActorLocation`)))
  (bind _returnvalue_x_2 (`KismetMathLibrary.BreakVector` (`self.K2_GetActorLocation`)))
  (if (`self.Is Dead`)
    (`self.K2_DestroyActor` :!label _label)
    (elif (<= _returnvalue_x (- (`self.Start location`) 800.0))
      (goto _label)
      (elif (>= _returnvalue_x_2 (+ (`self.Start location`) 800.0))
        (goto _label)))))

(event `self.DamageBox.OnComponentBeginOverlap`
  (params (OverlappedComponent :type "PrimitiveComponent Object Reference") (OtherActor :type "Actor Object Reference") (OtherComp :type "PrimitiveComponent Object Reference") (OtherBodyIndex :type Integer) (bFromSweep :type Boolean) (SweepResult :type "HitResult Structure (by ref)"))
  (`self.Damage Player` OtherActor OtherActor))

(event `self.PA_Health.OnHealthChanged`
  (params (HealthDelta :type "Float (single-precision)") (CurrentHealth :type "Float (single-precision)"))
  (`self.HandleOnHealthChanged` HealthDelta CurrentHealth))

(fn `Damage Player`
  (params (Object :type "Object Object Reference") (A :type "Object Object Reference"))
  (`/Engine/EditorBlueprintResources/StandardMacros.DoOnce` false
    (:`Completed`
      (if (`self.Is Dead`)
        _
        (elif (== A (`GameplayStatics.GetPlayerCharacter` 0))
          (bind _asbp_player (cast `/Game/Blueprints/BP_Player` Object))
          (`/Game/Blueprints/BP_Player.TakeDamage` _asbp_player (`self.Base Damage`))
          (`self.K2_DestroyActor`))))))

(fn `HandleOnHealthChanged`
  (params (HealthDelta :type "Float (single-precision)") (CurrentHealth :type "Float (single-precision)")))

(fn `UserConstructionScript`)

(fn `WallTakeDamage`
  (params (DamageTaken :type "Float (double-precision)"))
  (`PA_Health.ChangeHealth` (`self.PA_Health`) DamageTaken)
  (set `self.Is Dead` true))