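; Player character for a 2D flipbook platformer, with side-scrolling movement, jump, melee attack, parry, pause and level restart.
; Attacks enable an overlap box that damages enemies through a cast chain, while parries line-trace forward to knock back and damage Golems when ParryWindow is set.
; Tick picks locomotion flipbooks unless an action or death overrides them, and flipbook completion resets action states and DoOnce gates.
; HealthComponent events drive hurt reactions, and inputs report to a toggleable tutorial widget.
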(event `self.ReceiveBeginPlay`
  (add `PA_Health.OnHealthChanged` (`self.HealthComponent`) (`|CreateDelegate` :!event `HandleOnHealthChanged`))
  (add `PA_Health.OnDeath` (`self.HealthComponent`) (`|CreateDelegate` :!event `HandleOnDeath`))
  (add `PA_TutorialSubsystem.OnTutorialToggled` (subsystem `PA_TutorialSubsystem`) (delegate `TutorialStateUpdated`))
  (bind _asplayer_controller (cast `PlayerController` (`self.GetController`)))
  (`EnhancedInputSubsystemInterface.AddMappingContext` (pcsubsystem `EnhancedInputLocalPlayerSubsystem` _asplayer_controller) "/Game/Input/IMC_Platforming.IMC_Platforming" 0 (struct))
  (bind _returnvalue (`|CreateWidget` "/Game/Blueprints/UI/BP_PlayerHealthBar.BP_PlayerHealthBar_C" (`GameplayStatics.GetPlayerController` 0)))
  (`UserWidget.AddToViewport` _returnvalue 0)
  (`PrimitiveComponent.SetCollisionEnabled` (`self.Damagebox`) "NoCollision")
  (`self.CreateTutorial`))

(event `TutorialStateUpdated`
  (params (bTutorialState :type Boolean))
  (`self.UpdateTutorialVisibility` bTutorialState))

(event `Key|P`
  (params (Key :type "Key Structure"))
  (:`Pressed`
    (`GameplayStatics.SetGamePaused` true :!label _label)
    (bind _returnvalue (`|CreateWidget` "/Game/Blueprints/UI/BP_PauseMenu.BP_PauseMenu_C"))
    (`UserWidget.AddToViewport` _returnvalue 0)))

(event `Key|Escape`
  (params (Key :type "Key Structure"))
  (:`Pressed`
    (goto _label)))

(event `Key|Gamepad_FaceButton_Top`
  (params (Key :type "Key Structure"))
  (:`Pressed`
    (goto _label)))

(event `EnhancedInput|/Game/Input/Actions/IA_Jump`
  (params (ActionValue :type Boolean) (ElapsedSeconds :type "Float (double-precision)") (TriggeredSeconds :type "Float (double-precision)") (InputAction :type "InputAction Object Reference" :default "/Game/Input/Actions/IA_Jump.IA_Jump"))
  (:`Triggered`
    (`self.Jump`)
    (`/Game/Blueprints/UI/BP_TutorialSubtitles.JumpInputRegistered` (`self.TutorialWidget`)))
  (:`Completed`
    (`self.StopJumping`)))

(event `Key|R`
  (params (Key :type "Key Structure"))
  (:`Pressed`
    (`self.RestartLevel` :!label _label_2)))

(event `EnhancedInput|/Game/Input/Actions/IA_Move`
  (params (ActionValue :type "Float (double-precision)") (ElapsedSeconds :type "Float (double-precision)") (TriggeredSeconds :type "Float (double-precision)") (InputAction :type "InputAction Object Reference" :default "/Game/Input/Actions/IA_Move.IA_Move"))
  (:`Triggered`
    (`self.MovementAndRotation` ActionValue ActionValue ActionValue)
    (`/Game/Blueprints/UI/BP_TutorialSubtitles.MovementInputRegistered` (`self.TutorialWidget`))))

(event `Key|Gamepad_DPad_Up`
  (params (Key :type "Key Structure"))
  (:`Pressed`
    (goto _label_2)))

(event `self.HealthComponent.OnHealthChanged`
  (params (HealthDelta :type "Float (single-precision)") (CurrentHealth :type "Float (single-precision)"))
  (`self.HandleOnHealthChanged` HealthDelta CurrentHealth))

(event `self.ReceiveTick`
  (params (DeltaSeconds :type "Float (single-precision)"))
  (if (`self.IsDead`)
    _
    (elif (not (or (`self.IsAttacking`) (`self.IsParrying`) (`self.Taking Damage`)))
      (`self.UpdateAnimation`))))

(event `EnhancedInput|/Game/Input/Actions/IA_Parry`
  (params (ActionValue :type Boolean) (ElapsedSeconds :type "Float (double-precision)") (TriggeredSeconds :type "Float (double-precision)") (InputAction :type "InputAction Object Reference" :default "/Game/Input/Actions/IA_Parry.IA_Parry"))
  (:`Triggered`
    (`PaperFlipbookComponent.SetFlipbook` (`self.Sprite`) "/Game/PaperAssets/Knight_2D_Pixel_Art/Sprites/with_outline/Flipbooks/FB_Player_Defend.FB_Player_Defend")
    (`PaperFlipbookComponent.SetLooping` (`self.Sprite`) false)
    (set `self.IsParrying` true)
    (`/Engine/EditorBlueprintResources/StandardMacros.DoOnce` false :!label _label_3
      (:`Completed`
        (`self.ParryRaycast`)
        (`/Game/Blueprints/UI/BP_TutorialSubtitles.ParryInputRegistered` (`self.TutorialWidget`))))))

(event `ParryCooldown`
  (goto _label_3 :!via `Reset`))

(event `EnhancedInput|/Game/Input/Actions/IA_Attack`
  (params (ActionValue :type Boolean) (ElapsedSeconds :type "Float (double-precision)") (TriggeredSeconds :type "Float (double-precision)") (InputAction :type "InputAction Object Reference" :default "/Game/Input/Actions/IA_Attack.IA_Attack"))
  (:`Triggered`
    (`/Game/Blueprints/UI/BP_TutorialSubtitles.AttackInputRegistered` (`self.TutorialWidget`))
    (`/Engine/EditorBlueprintResources/StandardMacros.DoOnce` false :!label _label_4
      (:`Completed`
        (`PrimitiveComponent.SetCollisionEnabled` (`self.Damagebox`) "QueryOnly")
        (`PaperFlipbookComponent.SetFlipbook` (`self.Sprite`) "/Game/PaperAssets/Knight_2D_Pixel_Art/Sprites/with_outline/Flipbooks/FB_Player_Attack1.FB_Player_Attack1")
        (`PaperFlipbookComponent.SetLooping` (`self.Sprite`) false)
        (set `self.IsAttacking` true)
        (`SceneComponent.SetHiddenInGame` (`self.Damagebox`) false false)
        (if (not (`self.Contact`))
          (`PrimitiveComponent.SetCollisionEnabled` (`self.Damagebox`) "NoCollision"))))))

(event `Reset Attack`
  (goto _label_4 :!via `Reset`))

(event `self.Damagebox.OnComponentBeginOverlap`
  (params (OverlappedComponent :type "PrimitiveComponent Object Reference") (OtherActor :type "Actor Object Reference") (OtherComp :type "PrimitiveComponent Object Reference") (OtherBodyIndex :type Integer) (bFromSweep :type Boolean) (SweepResult :type "HitResult Structure (by ref)"))
  (set `self.Contact` true)
  (`KismetSystemLibrary.PrintString` (`KismetSystemLibrary.GetDisplayName` OtherActor))
  (`PrimitiveComponent.SetCollisionEnabled` (`self.Damagebox`) "NoCollision")
  (`self.ApplyDamage` OtherActor OtherActor OtherActor OtherActor OtherActor OtherActor))

(event `self.Sprite.OnFinishedPlaying`
  (if (not (`self.IsDead`))
    (`PaperFlipbookComponent.SetFlipbook` (`self.Sprite`) "/Game/PaperAssets/Knight_2D_Pixel_Art/Sprites/with_outline/Flipbooks/FB_Player_Idle.FB_Player_Idle")
    (`self.RestartAnimation`)
    (set `self.IsAttacking` false)
    (set `self.IsParrying` false)
    (set `self.Taking Damage` false)
    (`self.Reset Attack`)
    (`self.ParryCooldown`)
    (`SceneComponent.SetHiddenInGame` (`self.Damagebox`) true false)))

(fn `ApplyDamage`
  (params (DemonActor :type "Object Object Reference") (GolemActor :type "Object Object Reference") (ProjectileActor :type "Object Object Reference") (WizardActor :type "Object Object Reference") (FirewallActor :type "Object Object Reference") (FlyingActor :type "Object Object Reference"))
  (bind _asbp_fire_demon (cast `/Game/Blueprints/Characters/BP_FireDemon` DemonActor)
    (:`then`
      (`/Game/Blueprints/Characters/BP_FireDemon.DemonTakeDamage` _asbp_fire_demon (`self.Base Damage`)))
    (:`CastFailed`
      (bind _asbp_golem (cast `/Game/Blueprints/Characters/BP_Golem` FirewallActor)
        (:`then`
          (`/Game/Blueprints/Characters/BP_Golem.GolemTakeDamage` _asbp_golem (`self.Base Damage`)))
        (:`CastFailed`
          (bind _asbp_projectile (cast `/Game/Blueprints/Actors/BP_Projectile` GolemActor)
            (:`then`
              (`/Game/Blueprints/Actors/BP_Projectile.ProjectileTakeDamage` _asbp_projectile (`self.Base Damage`) null))
            (:`CastFailed`
              (bind _asbp_wizard (cast `/Game/Blueprints/Characters/BP_Wizard` ProjectileActor)
                (:`then`
                  (`/Game/Blueprints/Characters/BP_Wizard.WizardTakeDamage` _asbp_wizard (`self.Base Damage`)))
                (:`CastFailed`
                  (bind _asbp_fire_wall (cast `/Game/Blueprints/Actors/BP_FireWall` WizardActor)
                    (:`then`
                      (`/Game/Blueprints/Actors/BP_FireWall.WallTakeDamage` _asbp_fire_wall (`self.Base Damage`) null))
                    (:`CastFailed`
                      (bind _asbp_flying_demon (cast `/Game/Blueprints/Characters/BP_FlyingDemon` FlyingActor))
                      (`/Game/Blueprints/Characters/BP_FlyingDemon.FlyingTakeDamage` _asbp_flying_demon (`self.Base Damage`)))))))))))))

(fn `CreateTutorial`
  (bind _returnvalue (`|CreateWidget` "/Game/Blueprints/UI/BP_TutorialSubtitles.BP_TutorialSubtitles_C"))
  (set `self.TutorialWidget` _returnvalue)
  (`UserWidget.AddToViewport` _returnvalue 0)
  (if (`PA_TutorialSubsystem.GetTutorialToggle` (subsystem `PA_TutorialSubsystem`))
    (set `/Game/Blueprints/UI/BP_TutorialSubtitles.SubtitlesText` (`|MakeArray` "A and D to move around" "Space or W to Jump" "Left click to Attack" "Right click to Parry" :!type "Text") _returnvalue)
    (else
      (`PA_TutorialSubsystem.DisableTutorial` (subsystem `PA_TutorialSubsystem`)))))

(fn `HandleOnDeath`
  (`PaperFlipbookComponent.SetFlipbook` (`self.Sprite`) "/Game/PaperAssets/Knight_2D_Pixel_Art/Sprites/with_outline/Flipbooks/FB_Player_Death.FB_Player_Death")
  (`PaperFlipbookComponent.SetLooping` (`self.Sprite`) false)
  (set `self.IsDead` true)
  (`self.DisableInput` null)
  (bind _returnvalue (`|CreateWidget` "/Game/Maps/DeathScreen.DeathScreen_C"))
  (`UserWidget.AddToViewport` _returnvalue 0))

(fn `HandleOnHealthChanged`
  (params (`Health Delta` :type "Float (single-precision)") (CurrentHealth :type "Float (double-precision)"))
  (`PaperFlipbookComponent.SetFlipbook` (`self.Sprite`) "/Game/PaperAssets/Knight_2D_Pixel_Art/Sprites/with_outline/Flipbooks/FB_Player_Hurt.FB_Player_Hurt")
  (`PaperFlipbookComponent.SetLooping` (`self.Sprite`) false)
  (set `self.Taking Damage` true))

(fn `HitCheck`
  (for _array_element (`PrimitiveComponent.GetOverlappingActors` (`self.Damagebox`) "/Game/Blueprints/Characters/BP_Golem.BP_Golem_C")
    (`GameplayStatics.ApplyDamage` _array_element (`self.Base Damage`))))

(fn `MovementAndRotation`
  (params (A :type "Float (double-precision)") (A2 :type "Float (double-precision)") (ScaleValue :type "Float (single-precision)"))
  (if (> (`KismetMathLibrary.Abs` A) 0.1)
    (`self.AddMovementInput` (1.0 0.0 0.0) ScaleValue)
    (`Controller.SetControlRotation` (`self.GetController`) (select `bool` (> A2 0.0) :`false` (`KismetMathLibrary.MakeRotator` 0.0 0.0 180.0) :`true` (`KismetMathLibrary.MakeRotator` 0.0)))))

(fn `ParryRaycast`
  (bind _returnvalue (`self.K2_GetActorLocation`))
  (bind _outhit (`KismetSystemLibrary.LineTraceSingleByProfile` :`Start` _returnvalue :`End` (+ _returnvalue (* (`KismetMathLibrary.GetForwardVector` (`self.K2_GetActorRotation`)) (100.0 0.0 0.0))) :`ProfileName` "Enemy" :`DrawDebugType` "ForDuration" :`DrawTime` 1.0))
  (if (`self.ParryWindow`)
    (bind _asbp_golem (cast `/Game/Blueprints/Characters/BP_Golem` (`.HitActor` (`GameplayStatics.BreakHitResult` _outhit))))
    (`/Game/Blueprints/Characters/BP_Golem.HandleOnParried` _asbp_golem true 3000.0)
    (`/Game/Blueprints/Characters/BP_Golem.GolemTakeDamage` _asbp_golem (`self.Base Damage`))
    (set `self.ParryWindow` false)))

(fn `RestartAnimation`
  (`PaperFlipbookComponent.SetLooping` (`self.Sprite`) true)
  (if (not (`PaperFlipbookComponent.IsPlaying` (`self.Sprite`)))
    (`PaperFlipbookComponent.Play` (`self.Sprite`))))

(fn `RestartLevel`
  (`/Engine/EditorBlueprintResources/StandardMacros.DoOnce` false
    (:`Completed`
      (bind _returnvalue (`GameplayStatics.GetCurrentLevelName` true))
      (`GameplayStatics.OpenLevel` (`KismetStringLibrary.Conv_StringToName` _returnvalue)))))

(fn `TakeDamage`
  (params (DamageAmount :type "Float (double-precision)"))
  (`PA_Health.ChangeHealth` (`self.HealthComponent`) DamageAmount))

(fn `UpdateAnimation`
  (bind (_returnvalue_x _returnvalue_y _returnvalue_z) (`KismetMathLibrary.BreakVector` (`self.GetVelocity`)))
  (if (`NavMovementComponent.IsMovingOnGround` (`self.CharacterMovement`))
    (if (> (`KismetMathLibrary.VSize` (`self.GetVelocity`)) 0.0)
      (`PaperFlipbookComponent.SetFlipbook` (`self.Sprite`) "/Game/PaperAssets/Knight_2D_Pixel_Art/Sprites/with_outline/Flipbooks/FB_Player_Walk.FB_Player_Walk")
      (else
        (`PaperFlipbookComponent.SetFlipbook` (`self.Sprite`) "/Game/PaperAssets/Knight_2D_Pixel_Art/Sprites/with_outline/Flipbooks/FB_Player_Idle.FB_Player_Idle")))
    (elif (< _returnvalue_z -100.0)
      (`PaperFlipbookComponent.SetFlipbook` (`self.Sprite`) "/Game/PaperAssets/Knight_2D_Pixel_Art/Sprites/with_outline/Flipbooks/FP_Player_Fall.FP_Player_Fall")
      (else
        (`PaperFlipbookComponent.SetFlipbook` (`self.Sprite`) "/Game/PaperAssets/Knight_2D_Pixel_Art/Sprites/with_outline/Flipbooks/FB_Player_Rise.FB_Player_Rise")))))

(fn `UpdateTutorialVisibility`
  (params (Condition :type Boolean))
  (if Condition
    (`Widget.SetVisibility` (`self.TutorialWidget`) "Visible")
    (else
      (`Widget.SetVisibility` (`self.TutorialWidget`) "Collapsed")
      (set `/Game/Blueprints/UI/BP_TutorialSubtitles.SubtitleNumber` 0 (`self.TutorialWidget`)))))

(fn `UserConstructionScript`)