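; BP_FlyingDemon is a flipbook-animated flying enemy for side-view 2D play that swoops at the player.
; Tick holds hover height with a downward trace, closes in horizontally within vision range, then dives at the player's saved position and climbs back to recover.
; DamageBox is enabled for the swoop and gated to limit repeat hits.
; PAHealth events drive hurt and death, and movement uses fixed per-tick steps without delta time.
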(event `self.ReceiveBeginPlay`
  (add `PA_Health.OnHealthChanged` (`self.PA_Health`) (`|CreateDelegate` :!event `HandleOnHealthChanged`))
  (add `PA_Health.OnDeath` (`self.PA_Health`) (`|CreateDelegate` :!event `HandleOnDeath`))
  (`PrimitiveComponent.SetCollisionEnabled` (`self.DamageBox`) "NoCollision"))

(event `self.ReceiveTick`
  (params (DeltaSeconds :type "Float (single-precision)"))
  (bind (_returnvalue_x _returnvalue_y _returnvalue_z) (`KismetMathLibrary.BreakVector` (`self.GetPlayerLocation`)))
  (if (not (`self.IsDead`))
    (if (`self.HasSeenPlayer`)
      (if (`self.IsSwooping`)
        (`self.UpdateAttack`)
        (`self.FacePlayer`)
        (else
          (`self.EndAttack`)
          (`self.MaintainHeight`)
          (`self.FacePlayer`)
          (`KismetSystemLibrary.Delay` 3.0)
          (set `self.HasSeenPlayer` false)
          (set `self.IsRecovering` false)))
      (else
        (bind _returnvalue (`self.DistanceToPlayer`))
        (if _returnvalue
          (`self.StartAttack`)
          (else
            (`self.MaintainHeight`)
            (if (> (`self.VisionDistance`) (`self.GetDistanceToPlayer`))
              (if (not (`self.IsRecovering`))
                (`self.K2_SetActorTransform` (`KismetMathLibrary.MakeTransform` (+ (`self.K2_GetActorLocation`) (* (`KismetMathLibrary.Normal` (- (`KismetMathLibrary.MakeVector` _returnvalue_x _returnvalue_y _returnvalue_z) (`self.K2_GetActorLocation`))) (3.0 0.0 0.0)))))
                (`self.FacePlayer`)))))))
    (else
      (`/Engine/EditorBlueprintResources/StandardMacros.IsValid` (`self.HitBox`)
        (:`Is Valid`
          (`ActorComponent.K2_DestroyComponent` (`self.HitBox`))
          (`KismetSystemLibrary.Delay` 1.0)
          (`self.K2_DestroyActor`))))))

(event `self.DamageBox.OnComponentBeginOverlap`
  (params (OverlappedComponent :type "PrimitiveComponent Object Reference") (OtherActor :type "Actor Object Reference") (OtherComp :type "PrimitiveComponent Object Reference") (OtherBodyIndex :type Integer) (bFromSweep :type Boolean) (SweepResult :type "HitResult Structure (by ref)"))
  (`self.DamagePlayer` OtherActor OtherActor))

(event `self.PA_Health.OnHealthChanged`
  (params (HealthDelta :type "Float (single-precision)") (CurrentHealth :type "Float (single-precision)"))
  (`self.HandleOnHealthChanged` HealthDelta CurrentHealth))

(event `self.Sprite.OnFinishedPlaying`
  (if (not (`self.IsDead`))
    (`PaperFlipbookComponent.SetFlipbook` (`self.Sprite`) "/Game/PaperAssets/Flying_Demon_2D_Pixel_Art/Sprites/with_outline/Flipbooks/FB_FlyingDemon_Idle.FB_FlyingDemon_Idle")
    (`self.RestartAnimation`)))

(fn `DamagePlayer`
  (params (Object :type "Object Object Reference") (A :type "Object Object Reference"))
  (`/Engine/EditorBlueprintResources/StandardMacros.DoOnce` false
    (:`Completed`
      (if (`self.IsDead`)
        _
        (elif (== A (`GameplayStatics.GetPlayerCharacter` 0))
          (if (not (`self.StopDamage`))
            (bind _asbp_player (cast `/Game/Blueprints/Characters/BP_Player` Object))
            (`/Game/Blueprints/Characters/BP_Player.TakeDamage` _asbp_player (`self.BaseDamage`))
            (set `self.StopDamage` true)))))))

(fn `DistanceToPlayer`
  (returns (ReturnValue :type Boolean))
  (return (< (`self.GetDistanceToPlayer`) (`self.SwoopRange`))))

(fn `EndAttack`
  (if (not (< (`KismetMathLibrary.Vector_Distance` (`self.K2_GetActorLocation`) (`self.DestinationTargetLocation`)) (`self.DistanceToTargetTolerance`)))
    (`self.K2_SetActorTransform` (`KismetMathLibrary.MakeTransform` (+ (`self.K2_GetActorLocation`) (* (`KismetMathLibrary.Normal` (- (`self.DestinationTargetLocation`) (`self.K2_GetActorLocation`))) (5.0 0.0 5.0)))))
    (set `self.StopDamage` false)
    (`PrimitiveComponent.SetCollisionEnabled` (`self.DamageBox`) "NoCollision")))

(fn `FacePlayer`
  (bind _returnvalue_x (`KismetMathLibrary.BreakVector` (`self.K2_GetActorLocation`)))
  (bind _returnvalue_x_2 (`KismetMathLibrary.BreakVector` (`self.K2_GetActorLocation` (`GameplayStatics.GetPlayerCharacter` 0))))
  (if (> (- _returnvalue_x_2 _returnvalue_x) 0.0)
    (`self.K2_SetActorRotation` (struct :`Yaw` 180.0))
    (else
      (`self.K2_SetActorRotation` (struct)))))

(fn `FlyingTakeDamage`
  (params (`Damage Amount` :type "Float (double-precision)"))
  (`PA_Health.ChangeHealth` (`self.PA_Health`) `Damage Amount`))

(fn `GetDistanceToPlayer`
  (returns (Distance :type "Float (double-precision)"))
  (if (not (`KismetSystemLibrary.IsValid` (`self.CurrentPlayer`)))
    (bind _asbp_player (cast `/Game/Blueprints/Characters/BP_Player` (`GameplayStatics.GetPlayerCharacter` 0)))
    (set `self.CurrentPlayer` _asbp_player))
  (return (`KismetMathLibrary.Vector_Distance` (`self.K2_GetActorLocation`) (`self.K2_GetActorLocation` (`self.CurrentPlayer`)))))

(fn `GetPlayerLocation`
  (returns (ReturnValue :type "Vector Structure"))
  (if (`KismetSystemLibrary.IsValid` (`self.CurrentPlayer`))
    (return (`self.K2_GetActorLocation` (`self.CurrentPlayer`)))
    (else
      (bind _asbp_player (cast `/Game/Blueprints/Characters/BP_Player` (`GameplayStatics.GetPlayerCharacter` 0))
        (:`then`
          (bind _output_get (set `self.CurrentPlayer` _asbp_player))
          (return (`self.K2_GetActorLocation` _output_get)))
        (:`CastFailed`
          (return (0.0 0.0 0.0)))))))

(fn `HandleOnDeath`
  (`PaperFlipbookComponent.SetFlipbook` (`self.Sprite`) "/Game/PaperAssets/Flying_Demon_2D_Pixel_Art/Sprites/with_outline/Flipbooks/FB_FlyingDemon_Death.FB_FlyingDemon_Death")
  (`PaperFlipbookComponent.SetLooping` (`self.Sprite`) false)
  (set `self.IsDead` true))

(fn `HandleOnHealthChanged`
  (params (HealthDelta :type "Float (single-precision)") (CurrentHealth :type "Float (single-precision)"))
  (`PaperFlipbookComponent.SetFlipbook` (`self.Sprite`) "/Game/PaperAssets/Flying_Demon_2D_Pixel_Art/Sprites/with_outline/Flipbooks/FB_FlyingDemon_Hurt.FB_FlyingDemon_Hurt")
  (`PaperFlipbookComponent.SetLooping` (`self.Sprite`) false)
  (set `self.IsHurt` true))

(fn `IsFacingLeft`
  (returns (ReturnValue :type Boolean))
  (bind (_returnvalue_roll _returnvalue_pitch _returnvalue_yaw) (`KismetMathLibrary.BreakRotator` (`self.K2_GetActorRotation`)))
  (return (< _returnvalue_yaw 90.0)))

(fn `MaintainHeight`
  (bind (_outhit _returnvalue) (`KismetSystemLibrary.LineTraceSingleByProfile` :`Start` (`self.K2_GetActorLocation`) :`End` (- (`self.K2_GetActorLocation`) (`KismetMathLibrary.MakeVector` 0.0 0.0 (`self.FlyHeight`))) :`ProfileName` "BlockAllDynamic" :`DrawDebugType` "ForOneFrame"))
  (if (< (- (`self.FlyHeight`) (`.Distance` (`GameplayStatics.BreakHitResult` _outhit))) 6.0)
    _
    (elif _returnvalue
      (`self.K2_SetActorTransform` (`KismetMathLibrary.MakeTransform` (+ (`self.K2_GetActorLocation`) (0.0 0.0 2.0))))
      (else
        (`self.K2_SetActorTransform` (`KismetMathLibrary.MakeTransform` (+ (`self.K2_GetActorLocation`) (0.0 0.0 -2.0))))))))

(fn `RestartAnimation`
  (`PaperFlipbookComponent.SetLooping` (`self.Sprite`) true)
  (if (not (`PaperFlipbookComponent.IsPlaying` (`self.Sprite`)))
    (`PaperFlipbookComponent.Play` (`self.Sprite`))))

(fn `StartAttack`
  (bind (_returnvalue_x _returnvalue_y _returnvalue_z) (`KismetMathLibrary.BreakVector` (`self.GetPlayerLocation`)))
  (if (not (== (`PaperFlipbookComponent.GetFlipbook` (`self.Sprite`)) "/Game/PaperAssets/Flying_Demon_2D_Pixel_Art/Sprites/with_outline/Flipbooks/FB_FlyingDemon_Attack.FB_FlyingDemon_Attack"))
    (`PaperFlipbookComponent.SetFlipbook` (`self.Sprite`) "/Game/PaperAssets/Flying_Demon_2D_Pixel_Art/Sprites/with_outline/Flipbooks/FB_FlyingDemon_Attack.FB_FlyingDemon_Attack")
    (`PaperFlipbookComponent.SetLooping` (`self.Sprite`) false)
    (set `self.HasSeenPlayer` true)
    (set `self.AttackTargetLocation` (`KismetMathLibrary.MakeVector` _returnvalue_x 0.1 _returnvalue_z))
    (set `self.DestinationTargetLocation` (`self.K2_GetActorLocation`))
    (`PrimitiveComponent.SetCollisionEnabled` (`self.DamageBox`) "QueryOnly")
    (set `self.IsSwooping` true)))

(fn `UpdateAttack`
  (if (< (`KismetMathLibrary.Vector_Distance` (`self.K2_GetActorLocation`) (`self.AttackTargetLocation`)) (`self.DistanceToTargetTolerance`))
    (set `self.IsSwooping` false)
    (set `self.IsRecovering` true)
    (else
      (`self.K2_SetActorTransform` (`KismetMathLibrary.MakeTransform` (+ (`self.K2_GetActorLocation`) (* (`KismetMathLibrary.Normal` (- (`self.AttackTargetLocation`) (`self.K2_GetActorLocation`))) (5.0 0.0 5.0))))))))

(fn `UserConstructionScript`)